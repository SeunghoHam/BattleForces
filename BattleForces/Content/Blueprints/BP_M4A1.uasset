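; M4A1 rifle weapon Blueprint that handles fire and reload presentation for its owning BP_Character.
; OnFire and OnStartReload play matching montages together on the weapon, third-person body and first-person arms.
; Firing also spawns the shot sound at the muzzle socket, located through GetMuzzleLocation.
; A flag tracks the weapon's reload montage until completion or interruption, and IsReloading requires both it and the parent's result.
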(event EventBeginPlay
  (bind _asbp_character (Utilities|Casting|CastToBP_Character (Components|GetOwner)))
  (Variables|Default|SetOwnerCharacter _asbp_character))

(event Collision|EventActorBeginOverlap
  (params (OtherActor :type Actor%20Object%20Reference)))

(event EventTick
  (params (DeltaSeconds :type Float%20%28single-precision%29)))

(event EventOnFire
  (Development|PrintString "OnFire")
  (Utilities|FlowControl|Sequence
    (:then_0
      ;[1 1 1] M4A1 Fire몽타주
      (Animation|Montage|PlayMontage (Variables|Default|GetSkeletalMesh) "/Game/FPS_Assault_Pack/Animations/Rifle/A_Rifle_Shoot01_Montage.A_Rifle_Shoot01_Montage"
        (:then
          (bind _asbp_character (Utilities|Casting|CastToBP_Character (Components|GetOwner)))
          ;[1 1 1] 3인칭 Fire몽타주
          (Animation|Montage|PlayMontage (Variables|/Script/Engine.Character|GetMesh _asbp_character) "/Game/AnimStarterPack/Fire_Rifle_Hip_Montage.Fire_Rifle_Hip_Montage"
            (:then
              ;[1 1 1] 1인칭 Fire몽타주
              (Animation|Montage|PlayMontage (Variables|/Game/Blueprints/BP_Character.BP_Character_C|GetArm%20Mesh _asbp_character) "/Game/FPS_Assault_Pack/Animations/Rifle/A_Arms_Rifle_Shoot01_Montage.A_Arms_Rifle_Shoot01_Montage"))))))
    (:then_1
      ;[1 1 1] C++ 에서 GetMuzzleLocation 함수 만들어서 위치 연결시킬거
      (Audio|SpawnSoundatLocation "/Game/Sound/m4a1_Fire.m4a1_Fire" (CallFunction|GetMuzzleLocation) "0, 0, 0" 1.0 1.0 0.0 0 0))))

(event EventOnStartReload
  (Development|PrintString "OnStartReload")
  (Animation|Montage|PlayMontage (Variables|Default|GetSkeletalMesh) "/Game/FPS_Assault_Pack/Animations/Rifle/A_Rifle_Reload_Montage.A_Rifle_Reload_Montage"
    (:then
      (Variables|Default|SetIsPlayingReloadAnimation true)
      (bind _asbp_character (Utilities|Casting|CastToBP_Character (Components|GetOwner)))
      ;[1 1 1] 3인칭 Fire몽타주
      (Animation|Montage|PlayMontage (Variables|/Script/Engine.Character|GetMesh _asbp_character) "/Game/AnimStarterPack/Reload_Rifle_Hip_Montage.Reload_Rifle_Hip_Montage"
        (:then
          ;[1 1 1] 1인칭 Fire몽타주
          (Animation|Montage|PlayMontage (Variables|/Game/Blueprints/BP_Character.BP_Character_C|GetArm%20Mesh _asbp_character) "/Game/FPS_Assault_Pack/Animations/Rifle/A_Arms_Rifle_Reload_Montage.A_Arms_Rifle_Reload_Montage"))))
    (:OnCompleted
      (Variables|Default|SetIsPlayingReloadAnimation false :!label _label))
    (:OnInterrupted
      (goto _label))))

(fn ConstructionScript)

(fn GetMuzzleLocation
  (return (.location (Transformation|GetSocketTransform (Variables|Default|GetSkeletalMesh) "MuzzleSocket" "RTS_World"))))

(fn IsReloading
  (return (and (|CallParentFunction) (Variables|Default|GetIsPlayingReloadAnimation))))