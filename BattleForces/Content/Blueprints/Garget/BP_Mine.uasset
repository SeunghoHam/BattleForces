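; Mine gadget that sounds an audio alert while living enemy characters are inside its sphere; no explosion or damage logic is present.
; Tick polls sphere overlaps, comparing each character's team with the Instigator's, and plays Audio when one counts.
; The visibility trace starts and ends at the mine, and a zero count restarts playing audio instead of stopping it.
; Point damage destroys the mine, and EndPlay stops the audio.
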(event OnComponentBeginOverlap(Sphere)
  (params (OverlappedComponent :type Primitive%20Component%20Object%20Reference) (OtherActor :type Actor%20Object%20Reference) (OtherComp :type Primitive%20Component%20Object%20Reference) (OtherBodyIndex :type Integer) (bFromSweep :type Boolean) (SweepResult :type Hit%20Result%20Structure%20%28by%20ref%29)))

(event EventBeginPlay)

(event Collision|EventActorBeginOverlap
  (params (OtherActor :type Actor%20Object%20Reference)))

(event EventTick
  (params (DeltaSeconds :type Float%20%28single-precision%29))
  (bind _audio (Variables|Default|GetAudio))
  (bind _audio_2 (Variables|Default|GetAudio))
  (Variables|Default|SetEnemyCount 0)
  (for _array_element (Collision|GetOverlappingActors (Variables|Default|GetSphere) "/Script/Engine.Character" :!class /Script/Engine.PrimitiveComponent)
    ;[1 1 1] 캐릭터가 안죽었을 때만 감지에 포함
    (bind _asbase_character (Utilities|Casting|CastToBaseCharacter _array_element))
    (if (not (Variables|/Script/BattleForces.BaseCharacter|GetIsDead _asbase_character))
      (bind _asaotplayer_state (Utilities|Casting|CastToAOTPlayerState (Variables|/Script/Engine.Pawn|GetPlayerState _asbase_character)))
      (bind _asaotplayer_state_2 (Utilities|Casting|CastToAOTPlayerState (Variables|/Script/Engine.Pawn|GetPlayerState (Variables|Actor|GetInstigator))))
      (if (!= (Variables|/Script/BattleForces.AOTPlayerState|GetTeamId _asaotplayer_state_2) (Variables|/Script/BattleForces.AOTPlayerState|GetTeamId _asaotplayer_state))
        (bind _returnvalue (Collision|LineTraceByChannel (Transformation|GetActorLocation) (Transformation|GetActorLocation) "TraceTypeQuery1" false 0 "None"))
        (if (not _returnvalue)
          (Math|Integer|IncrementInt (Variables|Default|GetEnemyCount)
            (:%20%20
              (if (not (Audio|Components|Audio|IsPlaying _audio))
                (Audio|Components|Audio|Play _audio 0.0))))))))
  (if (== (Variables|Default|GetEnemyCount) 0)
    (if (Audio|Components|Audio|IsPlaying _audio_2)
      (Audio|Components|Audio|Play _audio_2 0.0))))

(event Game|Damage|EventPointDamage
  (params (Damage :type Float%20%28single-precision%29) (DamageType :type Damage%20Type%20Object%20Reference) (HitLocation :type Vector :default "0, 0, 0") (HitNormal :type Vector :default "0, 0, 0") (HitComponent :type Primitive%20Component%20Object%20Reference) (BoneName :type Name :default "None") (ShotFromDirection :type Vector :default "0, 0, 0") (InstigatedBy :type Controller%20Object%20Reference) (DamageCauser :type Actor%20Object%20Reference) (HitInfo :type Hit%20Result%20Structure%20%28by%20ref%29))
  (Actor|DestroyActor))

(event EventEndPlay
  (params (EndPlayReason :type EEndPlayReason%20Enum :default "Destroyed"))
  ;[1 1 1] 엑터가 사라질 때 이벤트
  (Audio|Components|Audio|Stop (Variables|Default|GetAudio)))

(fn ConstructionScript)