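; Game mode for a two-team, round-based AOT Defence match that handles team assignment, spawning and elimination wins.
; On login it parses the TeamInfo URL option, matching each player's unique ID to a team.
; FindPlayerStart picks a PlayerStart tagged with the team ID, falling back to the first one.
; Deaths accumulate until one team is fully dead, ending the round for the other; the list clears on WaitingToStart.
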(event Custom|OnPlayerDead
  (params (Player :type AOT%20Player%20State%20Object%20Reference))
  (Utilities|Array|Add (Variables|Default|GetDeathPlayerList) Player)
  (CallFunction|CheckRoundEnd))

(event EventOnSetMatchState
  (params (NewState :type Name :default "None"))
  ;[1 1 1] 상태 변화에 반응하는 이벤트
  (if (Utilities|Name|Equal(Name) NewState "WaitingToStart")
    (Utilities|Array|Clear (Variables|Default|GetDeathPlayerList))))

(event EventPostLogin
  (params (NewPlayer :type Player%20Controller%20Object%20Reference))
  (bind _optionsstring (Variables|Default|GetOptionsString))
  (bind _returnvalue (Class|GameplayStatics|ParseOption _optionsstring "TeamInfo"))
  (Development|PrintString (Variables|Default|GetOptionsString))
  (bind _asaotplayer_state (Utilities|Casting|CastToAOTPlayerState (Variables|/Script/Engine.Controller|GetPlayerState NewPlayer)))
  (if (not (Utilities|Enum|Equal(Enum) _returnvalue "0"))
    (bind _array_element (Utilities|Array|ForEachLoopwithBreak (Utilities|String|ParseIntoArray _returnvalue ",") :!label _label)
      (:LoopBody
        (if (Utilities|Enum|Equal(Enum) (.LeftS (Utilities|String|Split _array_element "@")) (Class|AOTPlayerState|GetUniqueIdString _asaotplayer_state))
          (Development|PrintString _array_element true true "(R=0.980180,G=1.000000,B=0.000000,A=1.000000)" 1e+01)
          (Class|AOTPlayerState|SetTeam _asaotplayer_state (Math|Conversions|ToInteger(Byte) (.RightS (Utilities|String|Split _array_element "@"))))
          (goto _label Break)))
      (:Completed
        (Development|PrintString (Utilities|String|ToString(Integer) (Variables|/Script/BattleForces.AOTPlayerState|GetTeamId _asaotplayer_state)))))))

(fn ConstructionScript)

(fn FindPlayerStart
  (params (Player :type Controller%20Object%20Reference) (IncomingName :type String))
  ;[1 1 1] 오버라이딩 함수
  (bind _asaotplayer_state (Utilities|Casting|CastToAOTPlayerState (Variables|/Script/Engine.Controller|GetPlayerState Player)))
  (bind _outactors (Actor|GetAllActorsOfClass "/Script/Engine.PlayerStart"))
  (for _array_element _outactors
    (if (Utilities|Name|Equal(Name) (Variables|/Script/Engine.PlayerStart|GetPlayerStartTag _array_element) (Utilities|String|StringToName (Utilities|String|ToString(Integer) (Variables|/Script/BattleForces.AOTPlayerState|GetTeamId _asaotplayer_state))))
      (return _array_element)))
  (bind _outactors_2 (Actor|GetAllActorsOfClass "/Script/Engine.PlayerStart"))
  (return (Utilities|Array|Get(acopy) _outactors_2)))

(fn CheckRoundEnd
  (Utilities|FlowControl|Sequence
    (:then_0
      (for _array_element (Variables|/Script/Engine.GameStateBase|GetPlayerArray (Game|GetGameState))
        (bind _asaotplayer_state (Utilities|Casting|CastToAOTPlayerState _array_element))
        (switch int (Variables|/Script/BattleForces.AOTPlayerState|GetTeamId _asaotplayer_state)
          (:0
            (Math|Integer|IncrementInt (LocalVariables|GetATeamPlayerCount)))
          (:1
            (Math|Integer|IncrementInt (LocalVariables|GetBTeamPlayerCount))))))
    (:then_1
      (for _array_element_2 (Variables|Default|GetDeathPlayerList)
        (switch int (Variables|/Script/BattleForces.AOTPlayerState|GetTeamId _array_element_2)
          (:0
            (Math|Integer|IncrementInt (LocalVariables|GetATeamDeathCount)))
          (:1
            (Math|Integer|IncrementInt (LocalVariables|GetBTeamDeathCount)))))
      (if (or (== (LocalVariables|GetATeamDeathCount) (LocalVariables|GetATeamPlayerCount)) (== (LocalVariables|GetBTeamDeathCount) (LocalVariables|GetBTeamPlayerCount)))
        (Class|AOTDefenceGameMode|EndRound (Math|Integer|SelectInt 1 0 (== (LocalVariables|GetATeamDeathCount) (LocalVariables|GetATeamPlayerCount))))))))