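; Player controller for the lobby that sets up the local player's lobby screen and name.
; On BeginPlay, for a local controller outside a dedicated server, it creates and shows WBP_Lobby with the mouse cursor visible.
; It then applies the player name stored in BP_AOTGameInstance through the SetName console command.
; RebuildPlayerList forwards refresh requests to the lobby widget when it is valid.
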(event EventBeginPlay
  (bind _returnvalue (Game|GetPlayerController 0))
  ;[1 1 1] 보통 데디 서버에서 실행될 일이..?
  (if (and (not (Networking|IsDedicatedServer)) (Pawn|IsLocalController))
    (bind _returnvalue_2 (UserInterface|CreateWidget "/Game/Blueprints/Widget/WBP_Lobby.WBP_Lobby_C" _returnvalue))
    (UserInterface|Viewport|AddtoViewport _returnvalue_2 0)
    (Variables|Default|SetLobbyWidget _returnvalue_2)
    (Variables|/Script/Engine.PlayerController|SetbShowMouseCursor _returnvalue true)
    (bind _asbp_aotgame_instance (Utilities|Casting|CastToBP_AOTGameInstance (Game|GetGameInstance)))
    (Development|ExecuteConsoleCommand (Utilities|String|Append "SetName" (Variables|/Game/Blueprints/BP_AOTGameInstance.BP_AOTGameInstance_C|GetPlayerName _asbp_aotgame_instance)) self)))

(event EventTick
  (params (DeltaSeconds :type Float%20%28single-precision%29)))

(fn ConstructionScript)

(fn RebuildPlayerList
  (bind _lobbywidget (Variables|Default|GetLobbyWidget))
  (Utilities|IsValid _lobbywidget
    (:Is%20Valid
      (Default|RebuildingPlayerList _lobbywidget))))